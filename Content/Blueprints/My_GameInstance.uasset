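; Game instance that creates and shows the game's UI screens: main menu, gameplay HUD, lose screen and pause menu.
; Each show event creates its widget for the first player controller only if the cached reference is invalid, then adds it to the viewport.
; The main menu and gameplay events also show the mouse cursor, and the gameplay widget is created with a starting electrical energy value.
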(event `ShowWB_MainMenu`
  ;[1 1 1] ShowMainMenu
  (`/Engine/EditorBlueprintResources/StandardMacros.IsValid` (`self.WB_Main_Menu`)
    (:`Is Valid`
      _)
    (:`Is Not Valid`
      (bind _returnvalue (`|CreateWidget` "/Game/UI/WB_MainMenu.WB_MainMenu_C" (`GameplayStatics.GetPlayerController` 0)))
      (set `self.WB_Main_Menu` _returnvalue)))
  (`UserWidget.AddToViewport` (`self.WB_Main_Menu`) 0)
  (set `PlayerController.bShowMouseCursor` true (`GameplayStatics.GetPlayerController` 0)))

(event `Show_WB_Gameplay`
  ;[1 1 1] ShowGamePlay
  (`/Engine/EditorBlueprintResources/StandardMacros.IsValid` (`self.WB_Gameplay`)
    (:`Is Valid`
      _)
    (:`Is Not Valid`
      (bind _returnvalue (`|CreateWidget` "/Game/UI/WB_Gameplay.WB_Gameplay_C" (`GameplayStatics.GetPlayerController` 0)))
      (set `self.WB_Gameplay` _returnvalue)))
  (`UserWidget.AddToViewport` (`self.WB_Gameplay`) 0)
  (set `PlayerController.bShowMouseCursor` true (`GameplayStatics.GetPlayerController` 0)))

(event `Show_WB_Lose`
  ;[1 1 1] ShowWBLose
  (`/Engine/EditorBlueprintResources/StandardMacros.IsValid` (`self.WB_Lose`)
    (:`Is Valid`
      _)
    (:`Is Not Valid`
      (bind _returnvalue (`|CreateWidget` "/Game/UI/WB_Lose.WB_Lose_C" (`GameplayStatics.GetPlayerController` 0)))
      (set `self.WB_Lose` _returnvalue)))
  (`UserWidget.AddToViewport` (`self.WB_Lose`) 0))

(event `ShowPauseMenu`
  ;[1 1 1] ShowPauseMenu
  (`/Engine/EditorBlueprintResources/StandardMacros.IsValid` (`self.WB_PauseMenu`)
    (:`Is Valid`
      _)
    (:`Is Not Valid`
      (bind _returnvalue (`|CreateWidget` "/Game/UI/WB_PauseMenu.WB_PauseMenu_C" (`GameplayStatics.GetPlayerController` 0)))
      (set `self.WB_PauseMenu` _returnvalue)))
  (`UserWidget.AddToViewport` (`self.WB_PauseMenu`) 0))